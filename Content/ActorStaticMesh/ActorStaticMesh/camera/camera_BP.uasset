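; Camera Blueprint that enables player input and tracks Left and Right key presses for yaw rotation.
; Key events set and clear two flags, and each new press prints a "Hello" debug string.
; Tick acts only when the flags differ, but only Right adds yaw input, scaled by a zero multiplier so no turn results.
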(event EventBeginPlay
  ;[1 1 1] このBPでのコントローラー入力を有効化
  (Input|EnableInput (Game|GetPlayerController 0)))

(event EventTick
  (params (DeltaSeconds :type Float%20%28single-precision%29))
  (bind _rightflag (Variables|Default|GetRightFlag))
  (bind _returnvalue (Math|Boolean|Equal(Boolean) _rightflag true))
  ;[1 1 1] キーが同時に押されてなければ
  (if (not (Math|Boolean|Equal(Boolean) _returnvalue (Math|Boolean|Equal(Boolean) (Variables|Default|GetLeftFlag) true)))
    (if _returnvalue
      (Pawn|Input|AddControllerYawInput (* 0.0 (Variables|Default|GetBaseTurnRate) (Utilities|Time|GetWorldDeltaSeconds))))))

(event Input|KeyboardEvents|Right
  (params (Key :type Key%20Structure :default "None"))
  ;[1 1 1] 左右キーの入力のフラグを管理する
  (:Pressed
    (if (Math|Boolean|Equal(Boolean) (Variables|Default|GetRightFlag) false)
      (Variables|Default|SetRightFlag true)
      (CallFunction|PrintText)))
  (:Released
    (if (Math|Boolean|Equal(Boolean) (Variables|Default|GetRightFlag) true)
      (Variables|Default|SetRightFlag false))))

(event Input|KeyboardEvents|Left
  (params (Key :type Key%20Structure :default "None"))
  ;[1 1 1] 左右キーの入力のフラグを管理する
  (:Pressed
    (if (Math|Boolean|Equal(Boolean) (Variables|Default|GetLeftFlag) false)
      (Variables|Default|SetLeftFlag true)
      (CallFunction|PrintText)))
  (:Released
    (if (Math|Boolean|Equal(Boolean) (Variables|Default|GetLeftFlag) true)
      (Variables|Default|SetLeftFlag false))))

(fn ConstructionScript
  (|CallParentFunction))

(fn PrintText
  (Development|PrintString "Hello"))